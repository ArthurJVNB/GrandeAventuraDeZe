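; BP_Agua builds a horizontal strip of animated water tiles at BeginPlay.
; It clamps the tile count, destroys tracked and attached tiles, then spawns evenly spaced BP_TileAnimada actors using the water sprite with die-on-collision enabled.
; Each tile gets a box collider with the "Agua" profile.
; Tiles are stored in an array and attached to this actor so they move and act as a group.
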(event `self.ReceiveBeginPlay`
  (`self.CriarTiles`))

(fn `CriarTiles`
  (locals (LocalHorizontalNum :type Integer))
  (set `local.LocalHorizontalNum` (`KismetMathLibrary.Max` (- (`self.TilesHorizontaisNum`) 1)))
  (`self.LimparTilesCriados`)
  (for _index (range (+ (`local.LocalHorizontalNum`) 1))
    ;[1 1 1] Criar os tiles e adicionar no array para utilização futura. Para facilitar movimentação e ações em grupo, todos os tiles criados são filhos dessa BP.
    (bind _returnvalue (`|SpawnActorFromClass` "/Game/Blueprints/Cenario/BP_TileAnimada.BP_TileAnimada_C" (`KismetMathLibrary.MakeTransform` (`KismetMathLibrary.MakeVector` (* _index 216.0))) "AlwaysSpawn" "OverrideRootScale" null "/Game/Imagens/Sprites/Elementos_Animados/SS_Water.SS_Water" true null))
    (bind _returnvalue_2 (`AddComponent|NODE_AddBoxComponent-1` :`self` _returnvalue))
    (`PrimitiveComponent.SetCollisionProfileName` _returnvalue_2 "Agua" true)
    (`BoxComponent.SetBoxExtent` _returnvalue_2 (750.0 750.0 750.0) true)
    (`KismetArrayLibrary.Array_Add` (`self.TilesCriados`) _returnvalue)
    (`self.K2_AttachToActor` _returnvalue self "None" "KeepRelative" "KeepRelative" "KeepRelative" false)))

(fn `LimparTilesCriados`
  (bind _outactors (`self.GetAttachedActors` true))
  (bind _tilescriados (`self.TilesCriados`))
  (`|ExecutionSequence`
    (:`then_0`
      ;[1 1 1] Destruir os tiles criados e limpar o array.
      (for _array_element _tilescriados
        (`self.K2_DestroyActor` _array_element))
      (`KismetArrayLibrary.Array_Clear` _tilescriados))
    (:`then_1`
      ;[1 1 1] Garantir que todos os tiles são destruidos.
      (for _array_element_2 _outactors :!label _label
        (`self.K2_DestroyActor` _array_element_2))
      (if (!= (`KismetArrayLibrary.Array_Length` _outactors) 0)
        (goto _label)))))

(fn `UserConstructionScript`)
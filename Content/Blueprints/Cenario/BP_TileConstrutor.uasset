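; BP_TileConstrutor is a scenery builder that spawns a grid of BP_TileEstatica tiles from horizontal and vertical counts.
; CriarTiles clamps the counts, clears previous tiles, then places tiles 256 units apart in X and downward Z, choosing top-row or lower-row left, middle and right sprites.
; Tiles are stored and attached for group handling; cleanup also destroys every attached actor.
; Neither BeginPlay nor the construction script runs the build.
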(event `self.ReceiveBeginPlay`)

(fn `CriarTiles`
  (locals (LocalVerticalNum :type Integer) (LocalHorizontalNum :type Integer))
  (bind _localhorizontalnum (`local.LocalHorizontalNum`))
  (set `local.LocalVerticalNum` (`KismetMathLibrary.Max` (- (`self.TilesVerticaisNum`) 1)))
  (set `local.LocalHorizontalNum` (`KismetMathLibrary.Max` (- (`self.TilesHorizontaisNum`) 1)))
  (`self.LimparTilesCriados`)
  (for _index (range (+ (`local.LocalVerticalNum`) 1))
    (for _index_2 (range (+ _localhorizontalnum 1))
      (bind _returnvalue (== _index_2 _localhorizontalnum))
      (bind _returnvalue_2 (== _index_2 0))
      ;[1 1 1] Criar os tiles e adicionar no array para utilização futura. Para facilitar movimentação e ações em grupo, todos os tiles criados são filhos dessa BP.
      (bind _returnvalue_3 (`|SpawnActorFromClass` "/Game/Blueprints/Cenario/BP_TileEstatica.BP_TileEstatica_C" (`KismetMathLibrary.MakeTransform` (`KismetMathLibrary.MakeVector` (* _index_2 256.0) 0.0 (* _index -256.0))) "AlwaysSpawn" "OverrideRootScale" null (select `bool` (== _index 0) :`false` (select `bool` _returnvalue_2 :`false` (select `bool` _returnvalue :`false` (`self.TileCentroMeio`) :`true` (`self.TileCentroDireita`)) :`true` (`self.TileCentroEsquerda`)) :`true` (select `bool` _returnvalue_2 :`false` (select `bool` _returnvalue :`false` (`self.TileMeio`) :`true` (`self.TileDireita`)) :`true` (`self.TileEsquerda`))) null))
      (`KismetArrayLibrary.Array_Add` (`self.TilesCriados`) _returnvalue_3)
      (`self.K2_AttachToActor` _returnvalue_3 self "None" "KeepRelative" "KeepRelative" "KeepRelative" false))))

(fn `LimparTilesCriados`
  (bind _outactors (`self.GetAttachedActors` true))
  (bind _tilescriados (`self.TilesCriados`))
  (`|ExecutionSequence`
    (:`then_0`
      ;[1 1 1] Destruir os tiles criados e limpar o array.
      (for _array_element _tilescriados
        (`self.K2_DestroyActor` _array_element))
      (`KismetArrayLibrary.Array_Clear` _tilescriados))
    (:`then_1`
      ;[1 1 1] Garantir que todos os tiles são destruidos.
      (for _array_element_2 _outactors :!label _label
        (`self.K2_DestroyActor` _array_element_2))
      (if (!= (`KismetArrayLibrary.Array_Length` _outactors) 0)
        (goto _label)))))

(fn `UserConstructionScript`)
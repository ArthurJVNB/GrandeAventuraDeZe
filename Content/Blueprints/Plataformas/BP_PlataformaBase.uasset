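; Base 2D side-scroller platform that can optionally destroy itself while the player stands on it.
; BeginPlay enables query collision only when UsaTemporizador is set, saving processing otherwise.
; Player overlap waits one second, then runs a Timeline tinting the sprite as warning alongside a timer that destroys the actor.
; End overlap clears the timer and restores the color, but does not cancel a pending Delay.
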(event `self.ReceiveBeginPlay`
  ;[1 1 1] Configura a caixa de colisão da plataforma, se for uma plataforma que some com o tempo liga a colisão, se não, desliga a colisão para economizar processamento.
  (`PrimitiveComponent.SetCollisionEnabled` (`self.Colisor`) (select `bool` (`self.bUsaTemporizador`) :`false` "NoCollision" :`true` "QueryOnly" :!type "ECollisionEnabled Enum")))

(event `self.Colisor.OnComponentBeginOverlap`
  (params (OverlappedComponent :type "PrimitiveComponent Object Reference") (OtherActor :type "Actor Object Reference") (OtherComp :type "PrimitiveComponent Object Reference") (OtherBodyIndex :type Integer) (bFromSweep :type Boolean) (SweepResult :type "HitResult Structure (by ref)"))
  ;[1 1 1] Se o jogador colidir com a plataforma, inicializa a contagem para destruição.
  (cast `/Game/Blueprints/Personagens/2DSideScrollerCharacter` OtherActor)
  (`self.InicializarTemporizador`))

(event `InicializarTemporizador`
  ;[1 1 1] Após um delay de 1 segundo, inicializa a animação que serve de feedback para o jogador saber que a plataforma será destruída. E inicializa a contagem regressiva para a destruição
  (`KismetSystemLibrary.Delay` 1.0)
  (`KismetSystemLibrary.K2_ClearAndInvalidateTimerHandle` (`self.Temporizador`))
  (`|ExecutionSequence`
    (:`then_0`
      (bind (_direction _cor) (`Timeline|Timeline_Temporizador` :!via `PlayFromStart`)
        (:`Update`
          (`PaperSpriteComponent.SetSpriteColor` (`self.PaperSprite`) _cor))))
    (:`then_1`
      (bind _returnvalue (`KismetSystemLibrary.K2_SetTimerDelegate` (delegate `DestruirPlataforma`) (`self.TempoParaDestruirPlataforma`)))
      (set `self.Temporizador` _returnvalue))))

(event `DestruirPlataforma`
  ;[1 1 1] Após um delay de 1 segundo, inicializa a animação que serve de feedback para o jogador saber que a plataforma será destruída. E inicializa a contagem regressiva para a destruição
  (`self.K2_DestroyActor`))

(event `self.Colisor.OnComponentEndOverlap`
  (params (OverlappedComponent :type "PrimitiveComponent Object Reference") (OtherActor :type "Actor Object Reference") (OtherComp :type "PrimitiveComponent Object Reference") (OtherBodyIndex :type Integer))
  ;[1 1 1] Se o jogador parar de colidir com a plataforma, para a contagem de destruição.
  (cast `/Game/Blueprints/Personagens/2DSideScrollerCharacter` OtherActor)
  (`self.CancelarTemporizador`))

(event `CancelarTemporizador`
  ;[1 1 1] Cancela e invalida o temporizador, para a animação de feedback de destruição e força a sprite a voltar para a cor original.
  (`KismetSystemLibrary.K2_ClearAndInvalidateTimerHandle` (`self.Temporizador`))
  (`TimelineComponent.Stop` (`self.Timeline_Temporizador`))
  (`PaperSpriteComponent.SetSpriteColor` (`self.PaperSprite`) (struct :`R` 1.0 :`G` 1.0 :`B` 1.0 :`A` 1.0)))

(fn `ConfigurarTamanho`
  ;[1 1 1] Configura o tamanho inicial da sprite.
  (`self.SetActorScale3D` (0.2 0.2 0.2)))

(fn `UserConstructionScript`
  (`self.ConfigurarTamanho`))
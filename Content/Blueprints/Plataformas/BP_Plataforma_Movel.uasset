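; BP_Plataforma_Movel is a moving platform that travels along a horizontal or vertical path, selected by EMovimentacaoTipo.
; On BeginPlay it stores its start location and plays the timeline for the selected movement type.
; Each timeline update calls Mover, which places the actor at the start location plus the animated value multiplied by Velocidade, without sweep.
; Velocidade therefore scales the travel offset rather than the timeline's playback rate.
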(event `self.ReceiveBeginPlay`
  ;[1 1 1] Inicializa a plataforma, salva a posição inicial e autoriza a plataforma a se mover.
  (`parent.ReceiveBeginPlay`)
  (set `self.PosicaoInicial` (`self.K2_GetActorLocation`))
  (`self.MoverPlataforma`))

(event `MoverPlataforma`
  ;[1 1 1] Controla o tipo de movimentação, horizontal ou vertical.
  (switch `/Game/Blueprints/Plataformas/EPlataformaMovimentacaoTipo` (`self.EMovimentacaoTipo`)
    (:`NewEnumerator0`
      (bind (_direction _animacao_horizontal) (`Timeline|Timeline_Horizontal` :!via `PlayFromStart`)
        (:`Update`
          (`self.Mover` _animacao_horizontal))))
    (:`NewEnumerator1`
      (bind (_direction_2 _animacao_vertical) (`Timeline|Timeline_Vertical` :!via `PlayFromStart`)
        (:`Update`
          (`self.Mover` _animacao_vertical))))))

(fn `Mover`
  (params (Valor :type "Vector Structure"))
  ;[1 1 1] Recebe a posição da animação e aplica no objeto multiplicado pela velocidade.
  (`self.K2_SetActorLocation` (+ (* Valor (`self.Velocidade`)) (`self.PosicaoInicial`))))

(fn `UserConstructionScript`
  (`parent.UserConstructionScript`))
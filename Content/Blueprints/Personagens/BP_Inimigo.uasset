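; BP_Inimigo is a flipbook-sprite enemy that patrols horizontally back and forth, takes damage and dies.
; A timeline offsets it from a saved start position, scaled by Velocidade; on finish it flips via negative X scale, re-saves position and restarts.
; SofrerDano removes one health, triggering either a timeline color flash or the death flipbook, which disables collision and destroys the actor when finished.
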(event `self.ReceiveBeginPlay`
  ;[1 1 1] Inicializa o inimigo e configura o tamanho da sprite.
  (`self.InicializarInimigo`)
  (`self.ConfigurarTamanho`))

(event `InicializarInimigo`
  ;[1 1 1] Configura a vida atual do inimigo, salva a posição inicial (para usar na movimentação), autoriza o inimigo a andar.
  (set `self.VidaAtual` (`self.VidaInicial`))
  (set `self.PosicaoInicial` (`self.K2_GetActorLocation`))
  (`self.Andar`))

(event `Andar`
  ;[1 1 1] Liga a animação de andar, ao chegar no fim da animação, inverter o lado que o inimigo está olhando e reinicia a animação.
  (bind (_direction `_movimentaçãohorizontalfrente`) (`Timeline|Timeline_Andar` :!via `PlayFromStart`)
    (:`Update`
      (`self.K2_SetActorLocation` (+ (* (* `_movimentaçãohorizontalfrente` (select `bool` (`self.bInverterSprite`) :`false` 1 :`true` -1)) (`self.Velocidade`)) (`self.PosicaoInicial`))))
    (:`Finished`
      (set `self.bInverterSprite` (not (`self.bInverterSprite`)))
      (`self.ConfigurarTamanho`)
      (set `self.PosicaoInicial` (`self.K2_GetActorLocation`))
      (`self.Andar`))))

(event `SofrerDanoAnim`
  (bind _sprite (`self.Sprite`))
  ;[1 1 1] Se o dano sofrido for o suficiente pra matar, troca a sprite para a animação de morte, após a animação terminar desliga o objeto.
  ; Se o dano sofrido não matar, chama a animação de feedback do inimigo.
  (if (<= (`self.VidaAtual`) 0)
    (`PaperFlipbookComponent.SetSpriteColor` _sprite (struct :`R` 1.0 :`G` 1.0 :`B` 1.0 :`A` 1.0))
    (`PaperFlipbookComponent.SetLooping` _sprite false)
    (`PaperFlipbookComponent.SetFlipbook` _sprite (`self.SS_Morrer`))
    (`PrimitiveComponent.SetCollisionEnabled` (`self.Colisor`) "NoCollision")
    (add `PaperFlipbookComponent.OnFinishedPlaying` _sprite (delegate `FimDaAnimacaoDeMorte`))
    (else
      (bind (_direction _mudarcor) (`Timeline|Timeline_Sofrer_Dano` :!via `PlayFromStart`)
        (:`Update`
          (`PaperFlipbookComponent.SetSpriteColor` (`self.Sprite`) _mudarcor))))))

(event `FimDaAnimacaoDeMorte`
  ;[1 1 1] Se o dano sofrido for o suficiente pra matar, troca a sprite para a animação de morte, após a animação terminar desliga o objeto.
  ; Se o dano sofrido não matar, chama a animação de feedback do inimigo.
  (`self.SetLifeSpan` 0.1))

(fn `ConfigurarTamanho`
  ;[1 1 1] Configura o tamanho inicial da sprite, baseado para o lugar que a sprite está olhando.
  (`self.SetActorScale3D` (`KismetMathLibrary.MakeVector` (`KismetMathLibrary.SelectFloat` -0.15 0.15 (`self.bInverterSprite`)) 0.15 0.15)))

(fn `Debug_Caminho_A_Ser_Feito`
  (bind (_returnvalue_x _returnvalue_y _returnvalue_z) (`KismetMathLibrary.BreakVector` (`self.K2_GetActorLocation`)))
  (`KismetSystemLibrary.DrawDebugLine` (`self.K2_GetActorLocation`) (`KismetMathLibrary.MakeVector` (* (select `bool` (`self.bInverterSprite`) :`false` -1 :`true` 1) (* (+ _returnvalue_x 60.0) (`self.Velocidade`))) _returnvalue_y _returnvalue_z) (struct :`R` 1.0 :`G` 0.109375 :`B` 0.109375 :`A` 1.0) 10.0 10.0))

(fn `SofrerDano`
  ;[1 1 1] Ao sofrer dano, diminui a vida e liga a animação de hit.
  (bind _result (`/Engine/EditorBlueprintResources/StandardMacros.DecrementInt` (`self.VidaAtual`))
    (:`  `
      (`self.SofrerDanoAnim`))))

(fn `UserConstructionScript`
  (`self.ConfigurarTamanho`))
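; BP_Item is a collectible sprite item, such as a spinning coin, that respawns after being collected.
; ItemColetado hides the active actor, clears EstaAtivo and starts a one-shot timer of TempoParaRenascer that calls Reaparecer to show and reactivate it.
; The construction script and BeginPlay both set a fixed small scale and randomize the flipbook start time so spins are out of sync.
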(event `self.ReceiveBeginPlay`
  ;[1 1 1] Configura o tamanho inicial da sprite. Adiciona um valor aleatório para começar a animação de giro da moeda.
  (`self.ConfigurarTamanho`)
  (`PaperFlipbookComponent.SetNewTime` (`self.Sprite`) (`KismetMathLibrary.RandomFloat`)))

(event `ItemColetado`
  ;[1 1 1] Ao colidir com o jogador, se o objeto está ativo, desliga o objeto e liga o temporizador para renascer.
  (if (`self.bEstaAtivo`)
    (`self.SetActorHiddenInGame` true)
    (`KismetSystemLibrary.K2_SetTimerDelegate` (delegate `Reaparecer`) (`self.TempoParaRenascer`))
    (set `self.bEstaAtivo` false)))

(event `Reaparecer`
  ;[1 1 1] Religa o objeto.
  (`self.SetActorHiddenInGame` false)
  (set `self.bEstaAtivo` true))

(fn `ConfigurarTamanho`
  ;[1 1 1] Configura o tamanho inicial da sprite.
  (`self.SetActorScale3D` (0.2 0.2 0.2)))

(fn `UserConstructionScript`
  ;[1 1 1] Configura o tamanho inicial da sprite. Adiciona um valor aleatório para começar a animação de giro da moeda.
  (`self.ConfigurarTamanho`)
  (`PaperFlipbookComponent.SetNewTime` (`self.Sprite`) (`KismetMathLibrary.RandomFloat`)))